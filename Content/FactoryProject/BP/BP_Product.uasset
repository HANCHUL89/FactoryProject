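; BP_Product is a factory product actor whose static mesh rides along a conveyor spline.
; On BeginPlay it finds a BP_ConveyorSpline, then each Tick advances a distance by MoveSpeed and places the mesh at that point with the spline's local-space rotation.
; Mesh overlap with a BP_StorageManager only stores a reference to it.
; A destroy-at-spline-end check exists but is disconnected, so it never runs.
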(event `self.ReceiveBeginPlay`
  (bind _returnvalue (`GameplayStatics.GetActorOfClass` "/Game/FactoryProject/BP/BP_ConveyorSpline.BP_ConveyorSpline_C"))
  (set `self.ConveyorSpline` _returnvalue))

(event `self.ReceiveTick`
  (params (DeltaSeconds :type "Float (single-precision)"))
  (bind _conveyorspline (`/Game/FactoryProject/BP/BP_ConveyorSpline.ConveyorSpline` (`self.ConveyorSpline`)))
  (if (`KismetSystemLibrary.IsValid` (`self.ConveyorSpline`))
    (bind _output_get (set `self.Distance` (+ (* DeltaSeconds (`self.MoveSpeed`)) (`self.Distance`))))
    (`SceneComponent.K2_SetWorldLocationAndRotation` (`self.StaticMesh`) (`SplineComponent.GetLocationAtDistanceAlongSpline` _conveyorspline _output_get "World") (`SplineComponent.GetRotationAtDistanceAlongSpline` _conveyorspline _output_get "Local") false false)))

(event `self.StaticMesh.OnComponentBeginOverlap`
  (params (OverlappedComponent :type "PrimitiveComponent Object Reference") (OtherActor :type "Actor Object Reference") (OtherComp :type "PrimitiveComponent Object Reference") (OtherBodyIndex :type Integer) (bFromSweep :type Boolean) (SweepResult :type "HitResult Structure (by ref)"))
  (bind _asbp_storage_manager (cast `/Game/FactoryProject/BP/BP_StorageManager` OtherActor))
  (set `self.StorageManagerRef` _asbp_storage_manager))

(fn `UserConstructionScript`)