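; BP_material is a factory material actor that moves its static mesh along a conveyor spline.
; BeginPlay stores the BP_ConveyorSpline1 found by GetActorOfClass as Test and resets Distance.
; Tick advances Distance by MoveSpeed and places the mesh on Test's spline, though its validity check reads a separate ConveyorSpline variable.
; End-of-spline destruction exists but is disconnected, so it never runs.
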(event `self.ReceiveBeginPlay`
  (bind _returnvalue (`GameplayStatics.GetActorOfClass` "/Game/FactoryProject/BP/BP_ConveyorSpline1.BP_ConveyorSpline1_C"))
  (set `self.Test` _returnvalue)
  (set `self.Distance` 0.0))

(event `self.ReceiveTick`
  (params (DeltaSeconds :type "Float (single-precision)"))
  (bind _conveyorspline (`/Game/FactoryProject/BP/BP_ConveyorSpline1.ConveyorSpline` (`self.Test`)))
  (if (`KismetSystemLibrary.IsValid` (`self.ConveyorSpline`))
    (bind _output_get (set `self.Distance` (+ (* DeltaSeconds (`self.MoveSpeed`)) (`self.Distance`))))
    (`SceneComponent.K2_SetWorldLocationAndRotation` (`self.StaticMesh`) (`SplineComponent.GetLocationAtDistanceAlongSpline` _conveyorspline _output_get "World") (`SplineComponent.GetRotationAtDistanceAlongSpline` _conveyorspline _output_get "World") false false)))

(fn `UserConstructionScript`)