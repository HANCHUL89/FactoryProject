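; BP_StorageManager is a storage manager that computes slot locations for a small grid in the world.
; On BeginPlay it reads the Arrow component's world location as the origin and fills GridLocations with a two-by-two layout at fixed spacing.
; Offsets follow world X and Y from the loop index, so the Arrow's rotation does not affect the grid.
; The file only builds the positions and does not use them.
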(event `self.ReceiveBeginPlay`
  (set `self.BaseLocation` (`SceneComponent.K2_GetComponentLocation` (`self.Arrow`)))
  (for _index (range 4)
    (`KismetArrayLibrary.Array_Add` (`self.GridLocations`) (`KismetMathLibrary.MakeVector` (+ (* (`KismetMathLibrary.Conv_IntToDouble` (`KismetMathLibrary.FFloor` (`KismetMathLibrary.Conv_IntToDouble` (/ _index 2)))) 100.0) (.x (`self.BaseLocation`))) (+ (.y (`self.BaseLocation`)) (`KismetMathLibrary.Conv_IntToDouble` (* (mod _index 2) 100))) (.z (`self.BaseLocation`))))))

(fn `UserConstructionScript`)