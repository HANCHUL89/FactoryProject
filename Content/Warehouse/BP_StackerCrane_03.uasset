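; Warehouse stacker crane that stores inbound pallets in empty PalletRack slots, moving on three axes with eased MoveComponentTo tweens.
; StartInbound finds a free slot, sends the crane to pickup position (row -1, level 0) and cycles the fork, whose overlap attaches the pallet.
; It then travels to the slot, extends, detaches the pallet, marks the slot full and retracts.
; Fixed delays and a timer coordinate the stages.
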(event `MoveZ`
  (params (Level :type Integer))
  (`KismetSystemLibrary.MoveComponentTo` (`self.LiftRoot`) (`KismetMathLibrary.MakeVector` 0.0 0.0 (`KismetMathLibrary.Conv_IntToDouble` (* Level 190))) (struct) true true 1.0))

(event `MoveX`
  (params (Row :type Integer) (Level :type Integer))
  (bind _location (`/Game/Warehouse/BP_PalletRack_02.GetSlotWorldLocation` (`self.PalletRack`) Row 0))
  (`KismetSystemLibrary.MoveComponentTo` (`self.CraneRoot`) (`KismetMathLibrary.MakeVector` (.x _location)) (struct) true true 1.0)
  (`self.MoveZ` Level))

(event `MoveXZ`
  (params (Row :type Integer) (Level :type Integer))
  (`|ExecutionSequence`
    (:`then_0`
      (`self.MoveX` Row Level))))

(event `MoveY`
  (bind (_relativelocation_x _relativelocation_y) (`KismetMathLibrary.BreakVector` (`SceneComponent.RelativeLocation` (`self.ForkRoot`))))
  (bind (_relativelocation_x_2 _relativelocation_y_2) (`KismetMathLibrary.BreakVector` (`SceneComponent.RelativeLocation` (`self.ForkRoot`))))
  (`KismetSystemLibrary.MoveComponentTo` (`self.ForkRoot`) (`KismetMathLibrary.MakeVector` 0.0 (+ _relativelocation_y_2 180.0)) (struct) true true 1.0)
  (`KismetSystemLibrary.MoveComponentTo` (`self.ForkRoot`) (`KismetMathLibrary.MakeVector` 0.0 (- _relativelocation_y 180.0)) (struct) true true 1.0))

(event `MoveYDetach`
  (params (Pallet :type "/Game/Warehouse/BP_Pallet Object Reference") (Index :type Integer))
  (bind (_relativelocation_x _relativelocation_y) (`KismetMathLibrary.BreakVector` (`SceneComponent.RelativeLocation` (`self.ForkRoot`))))
  (bind (_relativelocation_x_2 _relativelocation_y_2) (`KismetMathLibrary.BreakVector` (`SceneComponent.RelativeLocation` (`self.ForkRoot`))))
  (`KismetSystemLibrary.MoveComponentTo` (`self.ForkRoot`) (`KismetMathLibrary.MakeVector` 0.0 (+ _relativelocation_y_2 180.0)) (struct) true true 1.0)
  (`self.K2_DetachFromActor` Pallet "KeepWorld" "KeepWorld" "KeepWorld")
  (set `self.Pallet` null)
  (`/Game/Warehouse/BP_PalletRack_02.SetSlotFull` (`self.PalletRack`) Index true)
  (`KismetSystemLibrary.MoveComponentTo` (`self.ForkRoot`) (`KismetMathLibrary.MakeVector` 0.0 (- _relativelocation_y 180.0)) (struct) true true 1.0))

(event `self.ForkCollision.OnComponentBeginOverlap`
  (params (OverlappedComponent :type "PrimitiveComponent Object Reference") (OtherActor :type "Actor Object Reference") (OtherComp :type "PrimitiveComponent Object Reference") (OtherBodyIndex :type Integer) (bFromSweep :type Boolean) (SweepResult :type "HitResult Structure (by ref)"))
  (`|ExecutionSequence`
    (:`then_0`
      (bind _asbp_pallet (cast `/Game/Warehouse/BP_Pallet` OtherActor))
      (`self.AttachPallet` _asbp_pallet))))

(event `InboundMoveDetach`
  (params (Row :type Integer) (Level :type Integer) (Index :type Integer) (Pallet :type "/Game/Warehouse/BP_Pallet Object Reference"))
  (`self.MoveXZ` Row Level)
  (`KismetSystemLibrary.Delay` 1.0)
  (`self.MoveYDetach` Pallet Index))

(event `InboundMoveAttach`
  (`self.MoveXZ` -1)
  (`KismetSystemLibrary.K2_SetTimer` null "MoveY" 1.0))

(event `StartInbound`
  (params (Pallet :type "/Game/Warehouse/BP_Pallet Object Reference"))
  (bind _output_get (set `self.Pallet` Pallet))
  (bind (_find _row _level _index) (`/Game/Warehouse/BP_PalletRack_02.FindEmptySlot` (`self.PalletRack`)))
  (if _find
    (bind _output_get_2 (set `self.Row` _row))
    (bind _output_get_3 (set `self.Level` _level))
    (`self.InboundMoveAttach`)
    (`KismetSystemLibrary.Delay` 3.0)
    (`self.InboundMoveDetach` _output_get_2 _output_get_3 _index _output_get)
    (else
      (`KismetSystemLibrary.PrintString` "Finish" true true (struct :`G` 0.66 :`B` 1.0 :`A` 1.0) 10000.0))))

(fn `AttachPallet`
  (params (Pallet :type "/Game/Warehouse/BP_Pallet Object Reference"))
  (if (`KismetSystemLibrary.IsValid` Pallet)
    (`self.K2_AttachToComponent` Pallet (`self.Fork`) "None" "KeepWorld" "KeepWorld" "KeepWorld" false)
    (set `self.Pallet` Pallet)))

(fn `DetachPallet`
  (bind _pallet (`self.Pallet`))
  (if (`KismetSystemLibrary.IsValid` _pallet)
    (`self.K2_DetachFromActor` _pallet "KeepWorld" "KeepWorld" "KeepWorld")
    (set `self.Pallet` null)))

(fn `DoInbound`
  (params (Pallet :type "/Game/Warehouse/BP_Pallet Object Reference"))
  (returns (Row :type Integer) (Level :type Integer))
  (set `self.Pallet` Pallet)
  (bind (_find _row _level) (`/Game/Warehouse/BP_PalletRack_02.FindEmptySlot` (`self.PalletRack`)))
  (if _find
    (bind _output_get (set `self.Row` _row))
    (bind _output_get_2 (set `self.Level` _level))
    (return _output_get _output_get_2)))

(fn `UserConstructionScript`)