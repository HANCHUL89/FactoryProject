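; Warehouse stacker crane that attaches pallets with its fork and carries them to rack cells.
; Tick runs a MoveType state machine stepping crane, lift and fork roots through attach, travel, detach and inbound phases, using grid indices for targets.
; Fork overlap attaches the pallet.
; PickUpPallet starts a hardcoded rack move, immediately overridden by an inbound move if a pallet is held; crane and lift only move in positive directions.
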(event `self.ReceiveBeginPlay`
  (set `self.MoveType` "NewEnumerator4"))

(event `PickUpPallet`
  (`self.MoveToRack` 2 2)
  (if (`KismetSystemLibrary.IsValid` (`self.Pallet`))
    (`self.MoveToInbound` 0)))

(event `self.ReceiveTick`
  (params (DeltaSeconds :type "Float (single-precision)"))
  (switch `/Game/Warehouse/EN_MoveType` (`self.MoveType`)
    (:`NewEnumerator5`
      (`self.MoveAttachIn` DeltaSeconds))
    (:`NewEnumerator6`
      (`self.MoveAttachOut` DeltaSeconds))
    (:`NewEnumerator7`
      (`self.MoveRackX` DeltaSeconds))
    (:`NewEnumerator14`
      (`self.MoveRackZ` DeltaSeconds))
    (:`NewEnumerator15`
      (`self.MoveDetachIn` DeltaSeconds))
    (:`NewEnumerator16`
      (`self.MoveDetachOut` DeltaSeconds))
    (:`NewEnumerator1`
      (`self.MoveInboundZ` DeltaSeconds))
    (:`NewEnumerator0`
      (`self.MoveInboundX` DeltaSeconds))))

(event `self.ForkCollision.OnComponentBeginOverlap`
  (params (OverlappedComponent :type "PrimitiveComponent Object Reference") (OtherActor :type "Actor Object Reference") (OtherComp :type "PrimitiveComponent Object Reference") (OtherBodyIndex :type Integer) (bFromSweep :type Boolean) (SweepResult :type "HitResult Structure (by ref)"))
  (bind _asbp_pallet (cast `/Game/Warehouse/BP_Pallet` OtherActor))
  (`self.AttachPallet` _asbp_pallet))

(fn `AttachPallet`
  (params (Pallet :type "/Game/Warehouse/BP_Pallet Object Reference"))
  (if (`KismetSystemLibrary.IsValid` Pallet)
    (`self.K2_AttachToComponent` Pallet (`self.Fork`) "None" "KeepWorld" "KeepWorld" "KeepWorld" false)
    (set `self.Pallet` Pallet)))

(fn `DetachPallet`
  (bind _pallet (`self.Pallet`))
  (if (`KismetSystemLibrary.IsValid` _pallet)
    (`self.K2_DetachFromActor` _pallet "KeepWorld" "KeepWorld" "KeepWorld")
    (set `self.Pallet` null)))

(fn `MoveAttachIn`
  (params (DeltaTime :type "Float (double-precision)"))
  (bind (_relativelocation_x _relativelocation_y _relativelocation_z) (`KismetMathLibrary.BreakVector` (`SceneComponent.RelativeLocation` (`self.ForkRoot`))))
  (bind (_relativelocation_x_2 _relativelocation_y_2) (`KismetMathLibrary.BreakVector` (`SceneComponent.RelativeLocation` (`self.ForkRoot`))))
  (`SceneComponent.K2_SetRelativeLocation` (`self.ForkRoot`) (`KismetMathLibrary.MakeVector` _relativelocation_x (+ _relativelocation_y (* DeltaTime (`self.Speed`))) _relativelocation_z) false false)
  (if (>= _relativelocation_y_2 200.0)
    (set `self.MoveType` "NewEnumerator6")
    (`self.AttachPallet` null)))

(fn `MoveAttachOut`
  (params (DeltaTime :type "Float (double-precision)"))
  (bind (_relativelocation_x _relativelocation_y _relativelocation_z) (`KismetMathLibrary.BreakVector` (`SceneComponent.RelativeLocation` (`self.ForkRoot`))))
  (bind (_relativelocation_x_2 _relativelocation_y_2) (`KismetMathLibrary.BreakVector` (`SceneComponent.RelativeLocation` (`self.ForkRoot`))))
  (`SceneComponent.K2_SetRelativeLocation` (`self.ForkRoot`) (`KismetMathLibrary.MakeVector` _relativelocation_x (- _relativelocation_y (* DeltaTime (`self.Speed`))) _relativelocation_z) false false)
  (if (<= _relativelocation_y_2 0.0)
    (set `self.MoveType` "NewEnumerator7")))

(fn `MoveDetachIn`
  (params (DeltaTime :type "Float (double-precision)"))
  (bind (_relativelocation_x _relativelocation_y _relativelocation_z) (`KismetMathLibrary.BreakVector` (`SceneComponent.RelativeLocation` (`self.ForkRoot`))))
  (bind (_relativelocation_x_2 _relativelocation_y_2) (`KismetMathLibrary.BreakVector` (`SceneComponent.RelativeLocation` (`self.ForkRoot`))))
  (`SceneComponent.K2_SetRelativeLocation` (`self.ForkRoot`) (`KismetMathLibrary.MakeVector` _relativelocation_x (+ _relativelocation_y (* DeltaTime (`self.Speed`))) _relativelocation_z) false false)
  (if (>= _relativelocation_y_2 200.0)
    (set `self.MoveType` "NewEnumerator16")
    (`self.DetachPallet`)))

(fn `MoveDetachOut`
  (params (DeltaTime :type "Float (double-precision)"))
  (bind (_relativelocation_x _relativelocation_y _relativelocation_z) (`KismetMathLibrary.BreakVector` (`SceneComponent.RelativeLocation` (`self.ForkRoot`))))
  (bind (_relativelocation_x_2 _relativelocation_y_2) (`KismetMathLibrary.BreakVector` (`SceneComponent.RelativeLocation` (`self.ForkRoot`))))
  (`SceneComponent.K2_SetRelativeLocation` (`self.ForkRoot`) (`KismetMathLibrary.MakeVector` _relativelocation_x (- _relativelocation_y (* DeltaTime (`self.Speed`))) _relativelocation_z) false false)
  (if (<= _relativelocation_y_2 0.0)
    (set `self.MoveType` "NewEnumerator4")))

(fn `MoveInboundX`
  (params (DeltaTime :type "Float (double-precision)"))
  (bind (_relativelocation_x _relativelocation_y _relativelocation_z) (`KismetMathLibrary.BreakVector` (`SceneComponent.RelativeLocation` (`self.CraneRoot`))))
  (bind _relativelocation_x_2 (`KismetMathLibrary.BreakVector` (`SceneComponent.RelativeLocation` (`self.CraneRoot`))))
  (`SceneComponent.K2_SetRelativeLocation` (`self.CraneRoot`) (`KismetMathLibrary.MakeVector` (+ _relativelocation_x (* DeltaTime (`self.Speed`))) _relativelocation_y _relativelocation_z) false false)
  (if (>= _relativelocation_x_2 (* (`self.X`) 225.0))
    (set `self.MoveType` "NewEnumerator4")))

(fn `MoveInboundZ`
  (params (DeltaTime :type "Float (double-precision)"))
  (bind (_relativelocation_x _relativelocation_y _relativelocation_z) (`KismetMathLibrary.BreakVector` (`SceneComponent.RelativeLocation` (`self.LiftRoot`))))
  (bind (_relativelocation_x_2 _relativelocation_y_2 _relativelocation_z_2) (`KismetMathLibrary.BreakVector` (`SceneComponent.RelativeLocation` (`self.LiftRoot`))))
  (`SceneComponent.K2_SetRelativeLocation` (`self.LiftRoot`) (`KismetMathLibrary.MakeVector` _relativelocation_x_2 _relativelocation_y_2 (+ _relativelocation_z_2 (* DeltaTime (`self.Speed`)))) false false)
  (if (>= _relativelocation_z (* (`self.Z`) 190.0))
    (set `self.MoveType` "NewEnumerator0")))

(fn `MoveRackX`
  (params (DeltaTime :type "Float (double-precision)"))
  (bind (_relativelocation_x _relativelocation_y _relativelocation_z) (`KismetMathLibrary.BreakVector` (`SceneComponent.RelativeLocation` (`self.CraneRoot`))))
  (bind _relativelocation_x_2 (`KismetMathLibrary.BreakVector` (`SceneComponent.RelativeLocation` (`self.CraneRoot`))))
  (`SceneComponent.K2_SetRelativeLocation` (`self.CraneRoot`) (`KismetMathLibrary.MakeVector` (+ _relativelocation_x (* DeltaTime (`self.Speed`))) _relativelocation_y _relativelocation_z) false false)
  (if (>= _relativelocation_x_2 (* (`self.X`) 225.0))
    (set `self.MoveType` "NewEnumerator14")))

(fn `MoveRackZ`
  (params (DeltaTime :type "Float (double-precision)"))
  (bind (_relativelocation_x _relativelocation_y _relativelocation_z) (`KismetMathLibrary.BreakVector` (`SceneComponent.RelativeLocation` (`self.LiftRoot`))))
  (bind (_relativelocation_x_2 _relativelocation_y_2 _relativelocation_z_2) (`KismetMathLibrary.BreakVector` (`SceneComponent.RelativeLocation` (`self.LiftRoot`))))
  (`SceneComponent.K2_SetRelativeLocation` (`self.LiftRoot`) (`KismetMathLibrary.MakeVector` _relativelocation_x_2 _relativelocation_y_2 (+ _relativelocation_z_2 (* DeltaTime (`self.Speed`)))) false false)
  (if (>= _relativelocation_z (* (`self.Z`) 190.0))
    (set `self.MoveType` "NewEnumerator15")))

(fn `MoveToInbound`
  (params (X :type Integer) (Z :type Integer))
  (set `self.X` X)
  (set `self.Z` Z)
  (set `self.MoveType` "NewEnumerator1"))

(fn `MoveToRack`
  (params (X :type Integer) (Z :type Integer))
  (set `self.X` X)
  (set `self.Z` Z)
  (set `self.MoveType` "NewEnumerator5"))

(fn `UserConstructionScript`)