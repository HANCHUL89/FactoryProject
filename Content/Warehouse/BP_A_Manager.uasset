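; Warehouse manager actor that builds a grid of storage slots across levels and rows.
; On BeginPlay it clears and fills the Slots array with row, level and an initially false flag, then prints the count and a sample slot location as debug output.
; GetSlotWorldLocation offsets the slot origin component's world position by cell width along X and level height along Y, with Z fixed at zero.
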(event `self.ReceiveBeginPlay`
  (`KismetArrayLibrary.Array_Clear` (`self.Slots`))
  (for _index (range (`self.NumLevels`))
    (for _index_2 (range (`self.NumRows`))
      (bind _output_get (set `self.TempSlot` (make `/Game/Warehouse/ST_PalletSlot` _index_2 _index)))
      (`KismetArrayLibrary.Array_Add` (`self.Slots`) _output_get)))
  (`KismetSystemLibrary.PrintString` (`KismetStringLibrary.Conv_IntToString` (`KismetArrayLibrary.Array_Length` (`self.Slots`))))
  (bind _location (`self.GetSlotWorldLocation` 2 3))
  (`KismetSystemLibrary.PrintString` (`KismetStringLibrary.Conv_VectorToString` _location)))

(fn `GetSlotWorldLocation`
  (params (Row :type Integer) (Level :type Integer))
  (returns (Location :type "Vector Structure"))
  (bind (_returnvalue_x _returnvalue_y) (`KismetMathLibrary.BreakVector` (`SceneComponent.K2_GetComponentLocation` (`self.Comp_SlotOrigin`))))
  (return (`KismetMathLibrary.MakeVector` (+ _returnvalue_x (* (`KismetMathLibrary.Conv_IntToDouble` Row) (`self.CellWidth`))) (+ _returnvalue_y (* (`KismetMathLibrary.Conv_IntToDouble` Level) (`self.LevelHeight`))))))

(fn `UserConstructionScript`)