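; GM_Warehouse is the warehouse game mode that sets up the UI and tracks the clicked storage line.
; On BeginPlay it creates WBP_WarehouseUI, adds it to the viewport and shows the mouse cursor.
; OnclickStorageLine stores the passed storage line along with its crane, inbound manager and outbound manager as the current references.
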(event `self.ReceiveBeginPlay`
  (bind _returnvalue (`|CreateWidget` "/Game/Warehouse/UI/WBP_WarehouseUI.WBP_WarehouseUI_C"))
  (bind _output_get (set `self.WarehousuUI` _returnvalue))
  (`UserWidget.AddToViewport` _output_get 0)
  (set `PlayerController.bShowMouseCursor` true (`GameplayStatics.GetPlayerController` 0)))

(fn `OnclickStorageLine`
  (params (StorageLine :type "/Game/Warehouse/BP_StorageLine Object Reference"))
  (bind _output_get (set `self.StorageLine` StorageLine))
  (set `self.Crane` (`/Game/Warehouse/BP_StorageLine.Crane` _output_get))
  (set `self.InboundManager` (`/Game/Warehouse/BP_StorageLine.InboundManager` _output_get))
  (set `self.OutboundManager` (`/Game/Warehouse/BP_StorageLine.OutboundManager` _output_get)))

(fn `UserConstructionScript`)