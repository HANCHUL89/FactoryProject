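; Warehouse stacker crane that stores and retrieves BP_Pallet actors in rack slots for inbound and outbound jobs.
; Process functions pick a slot from the rack, or take a given one, then Tick runs an enum state machine moving crane, lift and fork one axis at a time.
; Fork overlap attaches pallets; the states detach them, update slot occupancy and notify the managers on completion.
; Tick also turns the crane's text label toward the camera.
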(event `self.ReceiveBeginPlay`
  (set `self.Jobtype` "NewEnumerator0"))

(event `self.ForkCollision.OnComponentBeginOverlap`
  (params (OverlappedComponent :type "PrimitiveComponent Object Reference") (OtherActor :type "Actor Object Reference") (OtherComp :type "PrimitiveComponent Object Reference") (OtherBodyIndex :type Integer) (bFromSweep :type Boolean) (SweepResult :type "HitResult Structure (by ref)"))
  (bind _asbp_pallet (cast `/Game/Warehouse/BP_Pallet` OtherActor))
  (set `self.Pallet` _asbp_pallet)
  (`self.AttachPallet`))

(event `self.ReceiveTick`
  (params (DeltaSeconds :type "Float (single-precision)"))
  (`SceneComponent.K2_SetWorldRotation` (`self.Txt_Crane`) (`KismetMathLibrary.FindLookAtRotation` (`SceneComponent.K2_GetComponentLocation` (`self.Txt_Crane`)) (`self.K2_GetActorLocation` (`GameplayStatics.GetPlayerCameraManager` 0))) false false)
  (switch `/Game/Warehouse/ENUM/EN_CraneJobType` (`self.Jobtype`)
    (:`NewEnumerator1`
      (`self.InboundMove` DeltaSeconds))
    (:`NewEnumerator2`
      (`self.OutboundMove` DeltaSeconds))))

(fn `AttachPallet`
  (bind _pallet (`self.Pallet`))
  (if (`KismetSystemLibrary.IsValid` _pallet)
    (`self.K2_AttachToComponent` _pallet (`self.Fork`) "None" "KeepWorld" "KeepWorld" "KeepWorld" false)
    (set `self.Pallet` _pallet)))

(fn `DetachPallet`
  (bind _pallet (`self.Pallet`))
  (if (`KismetSystemLibrary.IsValid` _pallet)
    (`self.K2_DetachFromActor` _pallet "KeepWorld" "KeepWorld" "KeepWorld")))

(fn `InboundMove`
  (params (InputPin :type "Float (single-precision)"))
  (bind _inboundmanager (`self.InboundManager`))
  (bind _relativelocation_x (`KismetMathLibrary.BreakVector` (`SceneComponent.RelativeLocation` (`self.CraneRoot`))))
  (bind (_relativelocation_x_2 _relativelocation_y _relativelocation_z) (`KismetMathLibrary.BreakVector` (`SceneComponent.RelativeLocation` (`self.LiftRoot`))))
  (bind (_relativelocation_x_3 _relativelocation_y_2) (`KismetMathLibrary.BreakVector` (`SceneComponent.RelativeLocation` (`self.ForkRoot`))))
  (bind (_relativelocation_x_4 _relativelocation_y_3) (`KismetMathLibrary.BreakVector` (`SceneComponent.RelativeLocation` (`self.ForkRoot`))))
  (bind (_relativelocation_x_5 _relativelocation_y_4 _relativelocation_z_2) (`KismetMathLibrary.BreakVector` (`SceneComponent.RelativeLocation` (`self.LiftRoot`))))
  (bind _relativelocation_x_6 (`KismetMathLibrary.BreakVector` (`SceneComponent.RelativeLocation` (`self.CraneRoot`))))
  (bind (_relativelocation_x_7 _relativelocation_y_5) (`KismetMathLibrary.BreakVector` (`SceneComponent.RelativeLocation` (`self.ForkRoot`))))
  (bind (_relativelocation_x_8 _relativelocation_y_6) (`KismetMathLibrary.BreakVector` (`SceneComponent.RelativeLocation` (`self.ForkRoot`))))
  (switch `/Game/Warehouse/ENUM/EN_InboundMoveType` (`self.InboundMoveType`)
    (:`NewEnumerator4`
      (set `self.Jobtype` "NewEnumerator0")
      (`/Game/Warehouse/BP_InboudManager.CompleteInbound` _inboundmanager)
      (`/Game/Warehouse/BP_InboudManager.CompleteInboundLog` _inboundmanager))
    (:`NewEnumerator5`
      (`self.MoveY_Fwd` InputPin)
      (if (>= _relativelocation_y_2 180.0)
        (set `self.InboundMoveType` "NewEnumerator6")))
    (:`NewEnumerator6`
      (`self.MoveY_Back` InputPin)
      (if (<= _relativelocation_y_3 0.0)
        (set `self.InboundMoveType` "NewEnumerator7")))
    (:`NewEnumerator7`
      (`self.MoveX_Left` InputPin)
      (if (>= _relativelocation_x_6 (* (`self.X`) 225.0))
        (set `self.InboundMoveType` "NewEnumerator14")))
    (:`NewEnumerator14`
      (`self.MoveZ_Up` InputPin)
      (if (>= _relativelocation_z (* (`self.Z`) 190.0))
        (set `self.InboundMoveType` "NewEnumerator15")))
    (:`NewEnumerator15`
      (`self.MoveY_Fwd` InputPin)
      (if (>= _relativelocation_y_6 180.0)
        (`self.DetachPallet`)
        (set `self.Pallet` null)
        (`/Game/Warehouse/BP_StorageSlot.SetSlotFull` (`self.PalleRack`) (`self.Index`) true)
        (set `self.InboundMoveType` "NewEnumerator16")
        (set `self.X` 0)
        (set `self.Z` 0)))
    (:`NewEnumerator16`
      (`self.MoveY_Back` InputPin)
      (if (<= _relativelocation_y_5 0.0)
        (set `self.InboundMoveType` "NewEnumerator1")))
    (:`NewEnumerator1`
      (`self.MoveZ_Down` InputPin)
      (if (<= _relativelocation_z_2 (* (`self.Z`) 190))
        (set `self.InboundMoveType` "NewEnumerator0")))
    (:`NewEnumerator0`
      (`self.MoveX_Right` InputPin)
      (if (<= _relativelocation_x (* (`self.X`) 225))
        (set `self.InboundMoveType` "NewEnumerator4")))))

(fn `InboundProcess`
  (bind (_find _x _z _index) (`/Game/Warehouse/BP_StorageSlot.FindEmptySlot` (`self.PalleRack`)))
  (if _find
    (set `self.X` _x)
    (set `self.Z` _z)
    (set `self.Index` _index)
    (set `self.Jobtype` "NewEnumerator1")
    (set `self.InboundMoveType` "NewEnumerator5")))

(fn `MoveX_Left`
  (params (DeltaTime :type "Float (double-precision)"))
  (bind (_relativelocation_x _relativelocation_y _relativelocation_z) (`KismetMathLibrary.BreakVector` (`SceneComponent.RelativeLocation` (`self.CraneRoot`))))
  (`SceneComponent.K2_SetRelativeLocation` (`self.CraneRoot`) (`KismetMathLibrary.MakeVector` (+ _relativelocation_x (* DeltaTime (`self.Speed`))) _relativelocation_y _relativelocation_z) false false))

(fn `MoveX_Right`
  (params (DeltaTime :type "Float (double-precision)"))
  (bind (_relativelocation_x _relativelocation_y _relativelocation_z) (`KismetMathLibrary.BreakVector` (`SceneComponent.RelativeLocation` (`self.CraneRoot`))))
  (`SceneComponent.K2_SetRelativeLocation` (`self.CraneRoot`) (`KismetMathLibrary.MakeVector` (- _relativelocation_x (* DeltaTime (`self.Speed`))) _relativelocation_y _relativelocation_z) false false))

(fn `MoveY_Back`
  (params (DeltaTime :type "Float (double-precision)"))
  (bind (_relativelocation_x _relativelocation_y _relativelocation_z) (`KismetMathLibrary.BreakVector` (`SceneComponent.RelativeLocation` (`self.ForkRoot`))))
  (`SceneComponent.K2_SetRelativeLocation` (`self.ForkRoot`) (`KismetMathLibrary.MakeVector` _relativelocation_x (- _relativelocation_y (* DeltaTime (`self.Speed`))) _relativelocation_z) false false))

(fn `MoveY_Fwd`
  (params (DeltaTime :type "Float (double-precision)"))
  (bind (_relativelocation_x _relativelocation_y _relativelocation_z) (`KismetMathLibrary.BreakVector` (`SceneComponent.RelativeLocation` (`self.ForkRoot`))))
  (`SceneComponent.K2_SetRelativeLocation` (`self.ForkRoot`) (`KismetMathLibrary.MakeVector` _relativelocation_x (+ _relativelocation_y (* DeltaTime (`self.Speed`))) _relativelocation_z) false false))

(fn `MoveZ_Down`
  (params (DeltaTime :type "Float (double-precision)"))
  (bind (_relativelocation_x _relativelocation_y _relativelocation_z) (`KismetMathLibrary.BreakVector` (`SceneComponent.RelativeLocation` (`self.LiftRoot`))))
  (`SceneComponent.K2_SetRelativeLocation` (`self.LiftRoot`) (`KismetMathLibrary.MakeVector` _relativelocation_x _relativelocation_y (- _relativelocation_z (* DeltaTime (`self.Speed`)))) false false))

(fn `MoveZ_Up`
  (params (DeltaTime :type "Float (double-precision)"))
  (bind (_relativelocation_x _relativelocation_y _relativelocation_z) (`KismetMathLibrary.BreakVector` (`SceneComponent.RelativeLocation` (`self.LiftRoot`))))
  (`SceneComponent.K2_SetRelativeLocation` (`self.LiftRoot`) (`KismetMathLibrary.MakeVector` _relativelocation_x _relativelocation_y (+ _relativelocation_z (* DeltaTime (`self.Speed`)))) false false))

(fn `OutboundMove`
  (params (InputPin :type "Float (single-precision)"))
  (bind _outboundmanager (`self.OutboundManager`))
  (bind (_relativelocation_x _relativelocation_y _relativelocation_z) (`KismetMathLibrary.BreakVector` (`SceneComponent.RelativeLocation` (`self.LiftRoot`))))
  (bind (_relativelocation_x_2 _relativelocation_y_2) (`KismetMathLibrary.BreakVector` (`SceneComponent.RelativeLocation` (`self.ForkRoot`))))
  (bind (_relativelocation_x_3 _relativelocation_y_3) (`KismetMathLibrary.BreakVector` (`SceneComponent.RelativeLocation` (`self.ForkRoot`))))
  (bind (_relativelocation_x_4 _relativelocation_y_4 _relativelocation_z_2) (`KismetMathLibrary.BreakVector` (`SceneComponent.RelativeLocation` (`self.LiftRoot`))))
  (bind _relativelocation_x_5 (`KismetMathLibrary.BreakVector` (`SceneComponent.RelativeLocation` (`self.CraneRoot`))))
  (bind _relativelocation_x_6 (`KismetMathLibrary.BreakVector` (`SceneComponent.RelativeLocation` (`self.CraneRoot`))))
  (bind _relativelocation_x_7 (`KismetMathLibrary.BreakVector` (`SceneComponent.RelativeLocation` (`self.CraneRoot`))))
  (bind (_relativelocation_x_8 _relativelocation_y_5) (`KismetMathLibrary.BreakVector` (`SceneComponent.RelativeLocation` (`self.ForkRoot`))))
  (bind (_relativelocation_x_9 _relativelocation_y_6) (`KismetMathLibrary.BreakVector` (`SceneComponent.RelativeLocation` (`self.ForkRoot`))))
  (switch `/Game/Warehouse/ENUM/EN_OutboundMoveType` (`self.OutboundMoveType`)
    (:`NewEnumerator1`
      (`self.MoveX_Left` InputPin)
      (if (>= _relativelocation_x_6 (* (`self.X`) 225.0))
        (set `self.OutboundMoveType` "NewEnumerator2")))
    (:`NewEnumerator2`
      (`self.MoveZ_Up` InputPin)
      (if (>= _relativelocation_z_2 (* (`self.Z`) 190.0))
        (set `self.OutboundMoveType` "NewEnumerator3")))
    (:`NewEnumerator3`
      (`self.MoveY_Fwd` InputPin)
      (if (>= _relativelocation_y_5 180.0)
        (set `self.OutboundMoveType` "NewEnumerator4")
        (`/Game/Warehouse/BP_StorageSlot.SetSlotFull` (`self.PalleRack`) (`self.Index`) false)))
    (:`NewEnumerator4`
      (`self.MoveY_Back` InputPin)
      (if (<= _relativelocation_y_2 0.0)
        (set `self.OutboundMoveType` "NewEnumerator5")
        (set `self.X` 6)
        (set `self.Z` 0)))
    (:`NewEnumerator5`
      (`self.MoveZ_Down` InputPin)
      (if (<= _relativelocation_z (* (`self.Z`) 190))
        (set `self.OutboundMoveType` "NewEnumerator6")))
    (:`NewEnumerator6`
      (`self.MoveX_Left` InputPin)
      (if (>= _relativelocation_x_5 (* (`self.X`) 225.0))
        (set `self.OutboundMoveType` "NewEnumerator7")))
    (:`NewEnumerator7`
      (`self.MoveY_Fwd` InputPin)
      (if (>= _relativelocation_y_3 180.0)
        (`self.DetachPallet`)
        (set `self.OutboundMoveType` "NewEnumerator8")))
    (:`NewEnumerator8`
      (`self.MoveY_Back` InputPin)
      (if (<= _relativelocation_y_6 0.0)
        (set `self.OutboundMoveType` "NewEnumerator9")
        (set `self.X` 0)))
    (:`NewEnumerator9`
      (`self.MoveX_Right` InputPin)
      (if (<= _relativelocation_x_7 (* (`self.X`) 225))
        (set `self.OutboundMoveType` "NewEnumerator0")))
    (:`NewEnumerator0`
      (set `self.Jobtype` "NewEnumerator0")
      (`/Game/Warehouse/BP_OutboundManager.CompleteOutbound` _outboundmanager)
      (`/Game/Warehouse/BP_OutboundManager.CompleteOutboundLog` _outboundmanager))))

(fn `OutboundProcess`
  (bind (_find _x _z _index) (`/Game/Warehouse/BP_StorageSlot.FindOccupiedSlot` (`self.PalleRack`)))
  (if _find
    (set `self.Index` _index)
    (set `self.X` _x)
    (set `self.Z` _z)
    (set `self.Jobtype` "NewEnumerator2")
    (set `self.OutboundMoveType` "NewEnumerator1")))

(fn `SelectOutboundProcess`
  (params (X :type Integer) (Z :type Integer) (Index :type Integer))
  (set `self.X` X)
  (set `self.Z` Z)
  (set `self.Index` Index)
  (set `self.Jobtype` "NewEnumerator2")
  (set `self.OutboundMoveType` "NewEnumerator1"))

(fn `UserConstructionScript`)