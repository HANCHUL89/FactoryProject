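; BP_PalletRack_02 is a warehouse pallet rack that tracks which slots in a five-by-five grid of rows and levels are full.
; BeginPlay initializes the flat Full array as empty and draws debug spheres at each slot position.
; Slot positions step from SlotOrigin along world X and Z, ignoring rack rotation.
; FindEmptySlot returns the first free row, level and index, and SetSlotFull updates occupancy.
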(event `self.ReceiveBeginPlay`
  (for _index (range 25)
    (`KismetArrayLibrary.Array_Set` (`self.Full`) _index false true))
  (for _index_2 (range 5)
    (for _index_3 (range 5)
      (bind _location (`self.GetSlotWorldLocation` _index_2 _index_3))
      (`KismetSystemLibrary.DrawDebugSphere` _location 50.0 12 (struct :`R` 1.0 :`G` 1.0 :`B` 1.0 :`A` 1.0) 100.0))))

(fn `FindEmptySlot`
  (returns (Find :type Boolean) (Row :type Integer) (Level :type Integer) (Index :type Integer))
  (for _index (range 25)
    (if (not (`|GetArrayItem` (`self.Full`) _index))
      (return true (/ _index 5) (mod _index 5) _index)))
  (return false -1 -1 -1))

(fn `GetSlotWorldLocation`
  (params (Row :type Integer) (Level :type Integer))
  (returns (Location :type "Vector Structure"))
  (bind (_returnvalue_x _returnvalue_y _returnvalue_z) (`KismetMathLibrary.BreakVector` (`SceneComponent.K2_GetComponentLocation` (`self.SlotOrigin`))))
  (return (`KismetMathLibrary.MakeVector` (+ (* Row (`self.PostX`)) _returnvalue_x) _returnvalue_y (+ (* Level (`self.PostZ`)) _returnvalue_z))))

(fn `SetSlotFull`
  (params (Index :type Integer) (Full :type Boolean))
  (`KismetArrayLibrary.Array_Set` (`self.Full`) Index Full))

(fn `UserConstructionScript`)