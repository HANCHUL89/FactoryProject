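; Test warehouse stacker crane that carries pallets into and out of rack slots on inbound and outbound jobs.
; Process functions pick a slot; Tick runs per-job state machines that move crane, lift and fork components along X, Z and Y.
; Fork overlap swaps pallet actors for a built-in mesh, and inbound storage picks rack side by index parity.
; Jobs update rack occupancy and notify their managers on completion.
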(event `self.ReceiveBeginPlay`
  (set `self.Jobtype` "NewEnumerator0")
  (`SceneComponent.SetVisibility` (`self.SM_Pallet`) false false))

(event `self.ForkCollision.OnComponentBeginOverlap`
  (params (OverlappedComponent :type "PrimitiveComponent Object Reference") (OtherActor :type "Actor Object Reference") (OtherComp :type "PrimitiveComponent Object Reference") (OtherBodyIndex :type Integer) (bFromSweep :type Boolean) (SweepResult :type "HitResult Structure (by ref)"))
  (bind _asbp_pallet_test (cast `/Game/Warehouse/BP_Pallet_Test` OtherActor))
  (`self.K2_DestroyActor` _asbp_pallet_test)
  (`SceneComponent.SetVisibility` (`self.SM_Pallet`) true false))

(event `self.ReceiveTick`
  (params (DeltaSeconds :type "Float (single-precision)"))
  (`SceneComponent.K2_SetWorldRotation` (`self.Txt_Crane`) (`KismetMathLibrary.FindLookAtRotation` (`SceneComponent.K2_GetComponentLocation` (`self.Txt_Crane`)) (`self.K2_GetActorLocation` (`GameplayStatics.GetPlayerCameraManager` 0))) false false)
  (switch `/Game/Warehouse/ENUM/EN_CraneJobType` (`self.Jobtype`)
    (:`NewEnumerator1`
      (`self.InboundMove` DeltaSeconds))
    (:`NewEnumerator2`
      (`self.OutboundMove` DeltaSeconds))))

(fn `AttachPallet`
  (bind _pallet (`self.Pallet`))
  (if (`KismetSystemLibrary.IsValid` _pallet)
    (`self.K2_AttachToComponent` _pallet (`self.Fork`) "None" "KeepWorld" "KeepWorld" "KeepWorld" false)
    (set `self.Pallet` _pallet)))

(fn `DetachPallet`
  (bind _pallet (`self.Pallet`))
  (if (`KismetSystemLibrary.IsValid` _pallet)
    (`self.K2_DetachFromActor` _pallet "KeepWorld" "KeepWorld" "KeepWorld")))

(fn `InboundMove`
  (params (InputPin :type "Float (single-precision)"))
  (bind _inboundmanager (`self.InboundManager`))
  (bind (_relativelocation_x _relativelocation_y _relativelocation_z) (`KismetMathLibrary.BreakVector` (`SceneComponent.RelativeLocation` (`self.LiftRoot`))))
  (bind (_relativelocation_x_2 _relativelocation_y_2) (`KismetMathLibrary.BreakVector` (`SceneComponent.RelativeLocation` (`self.ForkRoot`))))
  (bind (_relativelocation_x_3 _relativelocation_y_3 _relativelocation_z_2) (`KismetMathLibrary.BreakVector` (`SceneComponent.RelativeLocation` (`self.LiftRoot`))))
  (bind _relativelocation_x_4 (`KismetMathLibrary.BreakVector` (`SceneComponent.RelativeLocation` (`self.CraneRoot`))))
  (bind (_relativelocation_x_5 _relativelocation_y_4) (`KismetMathLibrary.BreakVector` (`SceneComponent.RelativeLocation` (`self.ForkRoot`))))
  (bind (_relativelocation_x_6 _relativelocation_y_5) (`KismetMathLibrary.BreakVector` (`SceneComponent.RelativeLocation` (`self.ForkRoot`))))
  (bind _relativelocation_x_7 (`KismetMathLibrary.BreakVector` (`SceneComponent.RelativeLocation` (`self.CraneRoot`))))
  (bind (_relativelocation_x_8 _relativelocation_y_6) (`KismetMathLibrary.BreakVector` (`SceneComponent.RelativeLocation` (`self.ForkRoot`))))
  (bind (_relativelocation_x_9 _relativelocation_y_7) (`KismetMathLibrary.BreakVector` (`SceneComponent.RelativeLocation` (`self.ForkRoot`))))
  (bind (_relativelocation_x_10 _relativelocation_y_8) (`KismetMathLibrary.BreakVector` (`SceneComponent.RelativeLocation` (`self.ForkRoot`))))
  (switch `/Game/Warehouse/EN_InboundTest` (`self.InboundMoveType`)
    (:`NewEnumerator1`
      (set `self.Jobtype` "NewEnumerator0")
      (`/Game/Warehouse/BP_InboudManager_Test.CompleteInbound` _inboundmanager)
      (`/Game/Warehouse/BP_InboudManager_Test.CompleteInboundLog` _inboundmanager))
    (:`NewEnumerator0`
      (`self.MoveY_Fwd` InputPin)
      (if (>= _relativelocation_y_6 250.0)
        (set `self.InboundMoveType` "NewEnumerator2")))
    (:`NewEnumerator2`
      (`self.MoveY_Back` InputPin)
      (if (<= _relativelocation_y_5 0.0)
        (set `self.InboundMoveType` "NewEnumerator3")))
    (:`NewEnumerator3`
      (`self.MoveX_Left` InputPin)
      (if (>= _relativelocation_x_4 (* (`self.X`) 250.0))
        (`self.MoveZ_Up` InputPin)
        (if (>= _relativelocation_z (* (`self.Z`) 250.0))
          (set `self.InboundMoveType` "NewEnumerator4"))))
    (:`NewEnumerator4`
      (if (== (mod (`self.Index`) 2) 0)
        (set `self.Move Y` "NewEnumerator1")
        (else
          (set `self.Move Y` "NewEnumerator0")))
      (switch `/Game/Warehouse/EN_MoveY` (`self.Move Y`)
        (:`NewEnumerator1`
          (`self.MoveY_Fwd` InputPin)
          (if (>= _relativelocation_y_7 250.0)
            (set `self.InboundMoveType` "NewEnumerator5")
            (`SceneComponent.SetVisibility` (`self.SM_Pallet`) false false)
            (`/Game/Warehouse/BP_StorageSlot_Test.SetSlotFull` (`self.PalleRack`) (`self.Index`) true)))
        (:`NewEnumerator0`
          (`self.MoveY_Back` InputPin)
          (if (<= _relativelocation_y_2 -250.0)
            (set `self.InboundMoveType` "NewEnumerator5")
            (`SceneComponent.SetVisibility` (`self.SM_Pallet`) false false)
            (`/Game/Warehouse/BP_StorageSlot_Test.SetSlotFull` (`self.PalleRack`) (`self.Index`) true)))))
    (:`NewEnumerator5`
      (if (== (mod (`self.Index`) 2) 0)
        (set `self.Move Y` "NewEnumerator1")
        (else
          (set `self.Move Y` "NewEnumerator0")))
      (switch `/Game/Warehouse/EN_MoveY` (`self.Move Y`)
        (:`NewEnumerator1`
          (`self.MoveY_Back` InputPin)
          (if (<= _relativelocation_y_8 0.0)
            (set `self.InboundMoveType` "NewEnumerator6")))
        (:`NewEnumerator0`
          (`self.MoveY_Fwd` InputPin)
          (if (>= _relativelocation_y_4 0.0)
            (set `self.InboundMoveType` "NewEnumerator6")))))
    (:`NewEnumerator6`
      (`self.MoveZ_Down` InputPin)
      (if (<= _relativelocation_z_2 0.0)
        (`self.MoveX_Right` InputPin)
        (if (<= _relativelocation_x_7 0.0)
          (set `self.InboundMoveType` "NewEnumerator1"))))))

(fn `InboundProcess`
  (bind (_find _x _z _index) (`/Game/Warehouse/BP_StorageSlot_Test.FindEmptySlot` (`self.PalleRack`)))
  (if _find
    (set `self.X` _x)
    (set `self.Z` _z)
    (set `self.Index` _index)
    (set `self.Jobtype` "NewEnumerator1")
    (set `self.InboundMoveType` "NewEnumerator0")))

(fn `MoveX_Left`
  (params (DeltaTime :type "Float (double-precision)"))
  (bind (_relativelocation_x _relativelocation_y _relativelocation_z) (`KismetMathLibrary.BreakVector` (`SceneComponent.RelativeLocation` (`self.CraneRoot`))))
  (`SceneComponent.K2_SetRelativeLocation` (`self.CraneRoot`) (`KismetMathLibrary.MakeVector` (`KismetMathLibrary.FClamp` (+ _relativelocation_x (* DeltaTime (`self.Speed`))) 0.0 (`KismetMathLibrary.Conv_IntToDouble` (* (`self.X`) 250))) _relativelocation_y _relativelocation_z) false false))

(fn `MoveX_Right`
  (params (DeltaTime :type "Float (double-precision)"))
  (bind (_relativelocation_x _relativelocation_y _relativelocation_z) (`KismetMathLibrary.BreakVector` (`SceneComponent.RelativeLocation` (`self.CraneRoot`))))
  (`SceneComponent.K2_SetRelativeLocation` (`self.CraneRoot`) (`KismetMathLibrary.MakeVector` (- _relativelocation_x (* DeltaTime (`self.Speed`))) _relativelocation_y _relativelocation_z) false false))

(fn `MoveY_Back`
  (params (DeltaTime :type "Float (double-precision)"))
  (bind (_relativelocation_x _relativelocation_y _relativelocation_z) (`KismetMathLibrary.BreakVector` (`SceneComponent.RelativeLocation` (`self.ForkRoot`))))
  (`SceneComponent.K2_SetRelativeLocation` (`self.ForkRoot`) (`KismetMathLibrary.MakeVector` _relativelocation_x (`KismetMathLibrary.FClamp` (- _relativelocation_y (* DeltaTime (`self.Speed`))) -250.0 250.0) _relativelocation_z) false false))

(fn `MoveY_Fwd`
  (params (DeltaTime :type "Float (double-precision)"))
  (bind (_relativelocation_x _relativelocation_y _relativelocation_z) (`KismetMathLibrary.BreakVector` (`SceneComponent.RelativeLocation` (`self.ForkRoot`))))
  (`SceneComponent.K2_SetRelativeLocation` (`self.ForkRoot`) (`KismetMathLibrary.MakeVector` _relativelocation_x (`KismetMathLibrary.FClamp` (+ _relativelocation_y (* DeltaTime (`self.Speed`))) -250.0 250.0) _relativelocation_z) false false))

(fn `MoveY_Test`
  (params (DeltaTime :type "Float (double-precision)"))
  (bind (_relativelocation_x _relativelocation_y) (`KismetMathLibrary.BreakVector` (`SceneComponent.RelativeLocation` (`self.ForkRoot`))))
  (bind (_relativelocation_x_2 _relativelocation_y_2) (`KismetMathLibrary.BreakVector` (`SceneComponent.RelativeLocation` (`self.ForkRoot`))))
  (bind (_relativelocation_x_3 _relativelocation_y_3 _relativelocation_z) (`KismetMathLibrary.BreakVector` (`SceneComponent.RelativeLocation` (`self.ForkRoot`))))
  (bind (_relativelocation_x_4 _relativelocation_y_4 _relativelocation_z_2) (`KismetMathLibrary.BreakVector` (`SceneComponent.RelativeLocation` (`self.ForkRoot`))))
  (if (== (mod (`self.Index`) 2) 0)
    (`SceneComponent.K2_SetRelativeLocation` (`self.ForkRoot`) (`KismetMathLibrary.MakeVector` _relativelocation_x_3 (`KismetMathLibrary.FClamp` (+ _relativelocation_y_3 (* DeltaTime (`self.Speed`))) 0.0 250.0) _relativelocation_z) false false)
    (if (>= _relativelocation_y 250.0)
      _)
    (else
      (`SceneComponent.K2_SetRelativeLocation` (`self.ForkRoot`) (`KismetMathLibrary.MakeVector` _relativelocation_x_4 (`KismetMathLibrary.FClamp` (- (* DeltaTime (`self.Speed`)) _relativelocation_y_4) 0.0 -250.0) _relativelocation_z_2) false false)
      (if (<= _relativelocation_y_2 -250.0)
        _))))

(fn `MoveZ_Down`
  (params (DeltaTime :type "Float (double-precision)"))
  (bind (_relativelocation_x _relativelocation_y _relativelocation_z) (`KismetMathLibrary.BreakVector` (`SceneComponent.RelativeLocation` (`self.LiftRoot`))))
  (`SceneComponent.K2_SetRelativeLocation` (`self.LiftRoot`) (`KismetMathLibrary.MakeVector` _relativelocation_x _relativelocation_y (`KismetMathLibrary.FClamp` (- _relativelocation_z (* DeltaTime (`self.Speed`))) 0.0 (`KismetMathLibrary.Conv_IntToDouble` (* (`self.Z`) 250)))) false false))

(fn `MoveZ_Up`
  (params (DeltaTime :type "Float (double-precision)"))
  (bind (_relativelocation_x _relativelocation_y _relativelocation_z) (`KismetMathLibrary.BreakVector` (`SceneComponent.RelativeLocation` (`self.LiftRoot`))))
  (`SceneComponent.K2_SetRelativeLocation` (`self.LiftRoot`) (`KismetMathLibrary.MakeVector` _relativelocation_x _relativelocation_y (`KismetMathLibrary.FClamp` (+ _relativelocation_z (* DeltaTime (`self.Speed`))) 0.0 (`KismetMathLibrary.Conv_IntToDouble` (* (`self.Z`) 250)))) false false))

(fn `OutboundMove`
  (params (InputPin :type "Float (single-precision)"))
  (bind _outboundmanager (`self.OutboundManager`))
  (bind (_relativelocation_x _relativelocation_y _relativelocation_z) (`KismetMathLibrary.BreakVector` (`SceneComponent.RelativeLocation` (`self.LiftRoot`))))
  (bind (_relativelocation_x_2 _relativelocation_y_2) (`KismetMathLibrary.BreakVector` (`SceneComponent.RelativeLocation` (`self.ForkRoot`))))
  (bind (_relativelocation_x_3 _relativelocation_y_3) (`KismetMathLibrary.BreakVector` (`SceneComponent.RelativeLocation` (`self.ForkRoot`))))
  (bind _relativelocation_x_4 (`KismetMathLibrary.BreakVector` (`SceneComponent.RelativeLocation` (`self.CraneRoot`))))
  (bind (_relativelocation_x_5 _relativelocation_y_4 _relativelocation_z_2) (`KismetMathLibrary.BreakVector` (`SceneComponent.RelativeLocation` (`self.LiftRoot`))))
  (bind _relativelocation_x_6 (`KismetMathLibrary.BreakVector` (`SceneComponent.RelativeLocation` (`self.CraneRoot`))))
  (bind _relativelocation_x_7 (`KismetMathLibrary.BreakVector` (`SceneComponent.RelativeLocation` (`self.CraneRoot`))))
  (bind (_relativelocation_x_8 _relativelocation_y_5) (`KismetMathLibrary.BreakVector` (`SceneComponent.RelativeLocation` (`self.ForkRoot`))))
  (bind (_relativelocation_x_9 _relativelocation_y_6) (`KismetMathLibrary.BreakVector` (`SceneComponent.RelativeLocation` (`self.ForkRoot`))))
  (switch `/Game/Warehouse/EN_OutboundTest` (`self.OutboundMoveType`)
    (:`NewEnumerator0`
      (set `self.Jobtype` "NewEnumerator0")
      (`/Game/Warehouse/BP_OutboundManager_Test.CompleteOutbound` _outboundmanager)
      (`/Game/Warehouse/BP_OutboundManager_Test.CompleteOutboundLog` _outboundmanager))
    (:`NewEnumerator1`
      (`self.MoveX_Left` InputPin)
      (if (>= _relativelocation_x_6 (* (`self.X`) 250.0))
        (`self.MoveZ_Up` InputPin)
        (if (>= _relativelocation_z_2 (* (`self.Z`) 250.0))
          (set `self.OutboundMoveType` "NewEnumerator2"))))
    (:`NewEnumerator2`
      (`self.MoveY_Fwd` InputPin)
      (if (>= _relativelocation_y_5 250.0)
        (`/Game/Warehouse/BP_StorageSlot_Test.SetSlotFull` (`self.PalleRack`) (`self.Index`) false)
        (set `self.OutboundMoveType` "NewEnumerator3")))
    (:`NewEnumerator3`
      (`self.MoveY_Back` InputPin)
      (if (<= _relativelocation_y_2 0.0)
        (set `self.OutboundMoveType` "NewEnumerator4")))
    (:`NewEnumerator4`
      (`self.MoveZ_Down` InputPin)
      (if (<= _relativelocation_z (* (`self.Z`) 250))
        (set `self.X` 4)
        (`self.MoveX_Left` InputPin)
        (if (>= _relativelocation_x_4 (* (`self.X`) 250.0))
          (set `self.OutboundMoveType` "NewEnumerator5"))))
    (:`NewEnumerator5`
      (`self.MoveY_Fwd` InputPin)
      (if (>= _relativelocation_y_3 250.0)
        (`self.DetachPallet`)
        (set `self.OutboundMoveType` "NewEnumerator6")))
    (:`NewEnumerator6`
      (`self.MoveY_Back` InputPin)
      (if (<= _relativelocation_y_6 0.0)
        (set `self.OutboundMoveType` "NewEnumerator7")))
    (:`NewEnumerator7`
      (`self.MoveX_Right` InputPin)
      (if (<= _relativelocation_x_7 0.0)
        (set `self.OutboundMoveType` "NewEnumerator0")))))

(fn `OutboundProcess`
  (bind (_find _x _z _index) (`/Game/Warehouse/BP_StorageSlot_Test.FindOccupiedSlot` (`self.PalleRack`)))
  (if _find
    (set `self.Index` _index)
    (set `self.X` _x)
    (set `self.Z` _z)
    (set `self.Jobtype` "NewEnumerator2")
    (set `self.OutboundMoveType` "NewEnumerator1")))

(fn `SelectOutboundProcess`
  (params (X :type Integer) (Z :type Integer) (Index :type Integer))
  (set `self.X` X)
  (set `self.Z` Z)
  (set `self.Index` Index)
  (set `self.Jobtype` "NewEnumerator2"))

(fn `UserConstructionScript`)