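; BP_StorageSlot_Test is a warehouse storage rack that lays out an X-by-Z grid of pallet slots and tracks which are full.
; The construction script adds paired PalletSlot and Pallet instances at each cell, offset either side of SlotOrigin along Y by GapY.
; A Full boolean array holds occupancy per slot, updated by SetSlotFull.
; FindEmptySlot and FindOccupiedSlot scan it linearly, returning the first match's index and grid coordinates.
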(fn `FindEmptySlot`
  (returns (Find :type Boolean) (X :type Integer) (Z :type Integer) (Index :type Integer))
  (for _index (range (* (* (`self.X`) (`self.Z`)) 2))
    (if (not (`|GetArrayItem` (`self.Full`) _index))
      (bind _returnvalue (/ _index 2))
      (return true (+ (/ _returnvalue (`self.X`)) 1) (mod _returnvalue (`self.X`)) _index)))
  (return false -1 -1 -1))

(fn `FindOccupiedSlot`
  (returns (Find :type Boolean) (X :type Integer) (Z :type Integer) (Index :type Integer))
  (for _index (range (* (* (`self.X`) (`self.Z`)) 2))
    (if (`|GetArrayItem` (`self.Full`) _index)
      (bind _returnvalue (/ _index 2))
      (return true (+ (/ _returnvalue (`self.X`)) 1) (mod _returnvalue (`self.X`)) _index)))
  (return false -1 -1 -1))

(fn `GetSlotWorldLocation`
  (params (X :type Integer) (Z :type Integer))
  (returns (Location :type "Vector Structure"))
  (bind (_returnvalue_x _returnvalue_y _returnvalue_z) (`KismetMathLibrary.BreakVector` (`SceneComponent.K2_GetComponentLocation` (`self.SlotOrigin`))))
  (return (`KismetMathLibrary.MakeVector` (+ (* X (`self.SlotSize`)) _returnvalue_x) _returnvalue_y (+ (* Z (`self.SlotSize`)) _returnvalue_z))))

(fn `SetSlotFull`
  (params (Index :type Integer) (Full :type Boolean))
  (`KismetArrayLibrary.Array_Set` (`self.Full`) Index Full))

(fn `UserConstructionScript`
  (locals (NewLocalVar :type "Rotator Structure" :default (struct)))
  (`InstancedStaticMeshComponent.ClearInstances` (`self.PalletSlot`))
  (for _index (range (* (`self.X`) (`self.Z`)))
    (bind _location (`self.GetSlotWorldLocation` (/ _index (`self.Z`)) (mod _index (`self.Z`))))
    (bind _x (.x _location))
    (bind _y (.y _location))
    (bind _z (.z _location))
    (bind _returnvalue (`KismetMathLibrary.MakeVector` _x (- _y (`self.GapY`)) _z))
    (`InstancedStaticMeshComponent.AddInstance` (`self.PalletSlot`) (`KismetMathLibrary.MakeTransform` _returnvalue (struct) (0.833 1.666 1.25)) true)
    (`InstancedStaticMeshComponent.AddInstance` (`self.Pallet`) (`KismetMathLibrary.MakeTransform` _returnvalue) true)
    (bind _returnvalue_2 (`KismetMathLibrary.MakeVector` _x (+ _y (`self.GapY`)) _z))
    (`InstancedStaticMeshComponent.AddInstance` (`self.PalletSlot`) (`KismetMathLibrary.MakeTransform` _returnvalue_2 (struct) (0.833 1.666 1.25)) true)
    (`InstancedStaticMeshComponent.AddInstance` (`self.Pallet`) (`KismetMathLibrary.MakeTransform` _returnvalue_2) true)))