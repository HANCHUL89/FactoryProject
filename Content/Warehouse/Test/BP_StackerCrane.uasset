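; BP_StackerCrane is a warehouse stacker crane that runs a slot retrieval motion toward an outbound point.
; MoveToSlot gets the slot location from AManagerRef, slides CraneBody along X, raises Lift, cycles Fork, lowers, moves the root to DetachPointRef and extends again.
; Steps are eased MoveComponentTo moves paced by fixed Delays.
; AttachPallet snaps pallets to Fork but is uncalled here, and a final retract is unwired.
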(event `MoveToSlot`
  (params (Row :type Integer) (Level :type Integer))
  (bind _returnvalue_x (`KismetMathLibrary.BreakVector` (`SceneComponent.K2_GetComponentLocation` (`self.DefaultSceneRoot`))))
  (bind _location (`/Game/Warehouse/Test/BP_PalletRack.GetSlotWorldLocation` (`self.A_ManagerRef`) Row Level))
  (`KismetSystemLibrary.MoveComponentTo` (`self.CraneBody`) (`KismetMathLibrary.MakeVector` (- (.x _location) _returnvalue_x)) (struct) true true 1.0)
  (`self.LiftToLevel` Level)
  (`KismetSystemLibrary.Delay` 1.0)
  (`self.ExtendFork`)
  (`KismetSystemLibrary.Delay` 1.0)
  (`self.RetrackFork`)
  (`KismetSystemLibrary.Delay` 1.0)
  (`self.LiftToLevel` 0)
  (`KismetSystemLibrary.Delay` 1.0)
  (`self.MoveDetachPoint`)
  (`KismetSystemLibrary.Delay` 1.0)
  (`self.ExtendFork`))

(event `ExtendFork`
  (`KismetSystemLibrary.MoveComponentTo` (`self.Fork`) (`KismetMathLibrary.MakeVector` 0.0 (+ (.y (`SceneComponent.RelativeLocation` (`self.Fork`))) (`self.ForkReachDisTance`))) (struct) true true 1.0)
  (`KismetSystemLibrary.Delay` 1.0))

(event `RetrackFork`
  (`KismetSystemLibrary.MoveComponentTo` (`self.Fork`) (`KismetMathLibrary.MakeVector` 0.0 (- (.y (`SceneComponent.RelativeLocation` (`self.Fork`))) (`self.ForkReachDisTance`))) (struct) true true 1.0))

(event `LiftToLevel`
  (params (Level :type Integer))
  (`KismetSystemLibrary.MoveComponentTo` (`self.Lift`) (`KismetMathLibrary.MakeVector` 0.0 0.0 (* (`KismetMathLibrary.Conv_IntToDouble` Level) (`self.LiftHeightPerLevel`))) (struct) true true 1.0)
  (`KismetSystemLibrary.Delay` 1.0))

(event `MoveDetachPoint`
  (bind (_returnvalue_x _returnvalue_y _returnvalue_z) (`KismetMathLibrary.BreakVector` (`SceneComponent.K2_GetComponentLocation` (`self.DefaultSceneRoot`))))
  (bind _returnvalue_x_2 (`KismetMathLibrary.BreakVector` (`SceneComponent.K2_GetComponentLocation` (`/Game/Warehouse/BP_OutboundManager.OutboundPoint` (`self.DetachPointRef`)))))
  (`KismetSystemLibrary.MoveComponentTo` (`self.DefaultSceneRoot`) (`KismetMathLibrary.MakeVector` _returnvalue_x_2 _returnvalue_y _returnvalue_z) (struct) true true 1.0)
  (`KismetSystemLibrary.Delay` 1.0))

(fn `AttachPallet`
  (params (Pallet :type "/Game/Warehouse/Test/BP_PalletSlot Object Reference"))
  (if (`KismetSystemLibrary.IsValid` (`self.Pallet`))
    (`self.K2_AttachToComponent` Pallet (`self.Fork`) "None" "SnapToTarget" "SnapToTarget" "KeepWorld" true)))

(fn `UserConstructionScript`)