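; Warehouse stacker crane test Blueprint that moves on three axes and picks up pallets.
; MoveX, MoveZ and MoveY ease the crane, lift and fork roots to relative targets over a fixed time.
; MoveToSlotLocation starts all three without waiting, feeding the target's Y to MoveZ and Z to MoveY.
; Fork overlap attaches any BP_Pallet to the fork, keeping world transform; no release logic exists, and SnapPalletToSlot is empty.
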(event `self.ReceiveBeginPlay`)

(event `MoveX`
  (params (TargetX :type "Float (double-precision)"))
  (`KismetSystemLibrary.MoveComponentTo` (`self.CraneRoot`) (`KismetMathLibrary.MakeVector` TargetX) (struct) true true 3.0))

(event `MoveZ`
  (params (TargetZ :type "Float (double-precision)"))
  (bind _liftroot (`self.LiftRoot`))
  (bind (_relativelocation_x _relativelocation_y) (`KismetMathLibrary.BreakVector` (`SceneComponent.RelativeLocation` _liftroot)))
  (`KismetSystemLibrary.MoveComponentTo` _liftroot (`KismetMathLibrary.MakeVector` _relativelocation_x _relativelocation_y TargetZ) (struct) true true 3.0))

(event `MoveY`
  (params (TargetY :type "Float (double-precision)"))
  (bind _forkroot (`self.ForkRoot`))
  (bind (_relativelocation_x _relativelocation_y _relativelocation_z) (`KismetMathLibrary.BreakVector` (`SceneComponent.RelativeLocation` _forkroot)))
  (`KismetSystemLibrary.MoveComponentTo` _forkroot (`KismetMathLibrary.MakeVector` _relativelocation_x TargetY _relativelocation_z) (struct) true true 3.0))

(event `self.ForkCollision.OnComponentBeginOverlap`
  (params (OverlappedComponent :type "PrimitiveComponent Object Reference") (OtherActor :type "Actor Object Reference") (OtherComp :type "PrimitiveComponent Object Reference") (OtherBodyIndex :type Integer) (bFromSweep :type Boolean) (SweepResult :type "HitResult Structure (by ref)"))
  (bind _asbp_pallet (cast `/Game/Warehouse/BP_Pallet` OtherActor))
  (`self.K2_AttachToComponent` _asbp_pallet (`self.ForkRoot`) "None" "KeepWorld" "KeepWorld" "KeepWorld" true))

(fn `MoveToSlotLocation`
  (params (TargetLocation :type "Vector Structure"))
  (`self.MoveX` (.x TargetLocation))
  (`self.MoveZ` (.y TargetLocation))
  (`self.MoveY` (.z TargetLocation)))

(fn `SnapPalletToSlot`)

(fn `UserConstructionScript`)