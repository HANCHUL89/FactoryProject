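; BP_PalletRack is a warehouse test actor that models a pallet rack as a grid of slots served by a stacker crane.
; GetSlotWorldLocation maps row and level to world X and Z from the CompSlotOrigin component.
; MoveCraneToSlot forwards row and level to StackerCraneRef.
; The logic that fills Slots, spawns BP_PalletSlot actors and test-moves the crane is unconnected, and BeginPlay is empty.
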(event `MoveCraneToSlot`
  (params (Row :type Integer) (Level :type Integer))
  (`/Game/Warehouse/Test/BP_StackerCrane_Test_01.MoveToSlot` (`self.StackerCraneRef`) Row Level))

(event `self.ReceiveBeginPlay`)

(fn `GetSlotWorldLocation`
  (params (Row :type Integer) (Level :type Integer))
  (returns (Location :type "Vector Structure"))
  (bind (_returnvalue_x _returnvalue_y _returnvalue_z) (`KismetMathLibrary.BreakVector` (`SceneComponent.K2_GetComponentLocation` (`self.Comp_SlotOrigin`))))
  (return (`KismetMathLibrary.MakeVector` (+ (* (`KismetMathLibrary.Conv_IntToDouble` Row) (`self.CellWidth`)) _returnvalue_x) _returnvalue_y (+ (* (`KismetMathLibrary.Conv_IntToDouble` Level) (`self.LevelHeight`)) _returnvalue_z))))

(fn `UserConstructionScript`)