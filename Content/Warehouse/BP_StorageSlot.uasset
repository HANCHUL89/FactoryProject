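; BP_StorageSlot is a warehouse storage rack that tracks which slots in a 5x5 grid of rows and levels are occupied.
; The construction script adds one indicator instance per slot, positioned from SlotOrigin using PostX and PostZ spacing.
; Linear searches return the first empty or occupied slot with its flat index, one-based row and zero-based level.
; SetSlotFull updates the Full array and flags the matching indicator through per-instance custom data.
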(event `self.ReceiveBeginPlay`
  (for _index (range 25)
    (`KismetArrayLibrary.Array_Set` (`self.Full`) _index false true)))

(fn `FindEmptySlot`
  (returns (Find :type Boolean) (X :type Integer) (Z :type Integer) (Index :type Integer))
  (for _index (range 25)
    (if (not (`|GetArrayItem` (`self.Full`) _index))
      (return true (+ (/ _index 5) 1) (mod _index 5) _index)))
  (return false -1 -1 -1))

(fn `FindOccupiedSlot`
  (returns (Find :type Boolean) (X :type Integer) (Z :type Integer) (Index :type Integer))
  (for _index (range 25)
    (if (`|GetArrayItem` (`self.Full`) _index)
      (return true (+ (/ _index 5) 1) (mod _index 5) _index)))
  (return false -1 -1 -1))

(fn `FireEvent`)

(fn `GetSlotWorldLocation`
  (params (Row :type Integer) (Level :type Integer))
  (returns (Location :type "Vector Structure"))
  (bind (_returnvalue_x _returnvalue_y _returnvalue_z) (`KismetMathLibrary.BreakVector` (`SceneComponent.K2_GetComponentLocation` (`self.SlotOrigin`))))
  (return (`KismetMathLibrary.MakeVector` (+ (* Row (`self.PostX`)) _returnvalue_x) _returnvalue_y (+ (* Level (`self.PostZ`)) _returnvalue_z))))

(fn `SetSlotFull`
  (params (Index :type Integer) (Full :type Boolean))
  (`KismetArrayLibrary.Array_Set` (`self.Full`) Index Full)
  (if Full
    (`InstancedStaticMeshComponent.SetCustomDataValue` (`self.SlotIndicators`) Index 0 1.0 false)
    (else
      (`InstancedStaticMeshComponent.SetCustomDataValue` (`self.SlotIndicators`) Index 0 0.0 false))))

(fn `UserConstructionScript`
  (`InstancedStaticMeshComponent.ClearInstances` (`self.SlotIndicators`))
  (for _index (range 5)
    (for _index_2 (range 5)
      (bind _location (`self.GetSlotWorldLocation` _index _index_2))
      (`InstancedStaticMeshComponent.AddInstance` (`self.SlotIndicators`) (`KismetMathLibrary.MakeTransform` _location (struct) (1.5 0.5 0.1)) false))))