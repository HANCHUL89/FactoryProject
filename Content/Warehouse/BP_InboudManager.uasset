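; Warehouse inbound manager that spawns pallets at a spawn point, sends them to the inbound point and coordinates with the crane.
; RequestInbound either switches the crane's job type or queues a pending request, depending on its current job.
; A looping timer spawns queued pallets when the slot is free and the crane's inbound state matches.
; A pallet entering the trigger frees the slot after a delay and conditionally starts the crane's InboundProcess.
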(event `self.ReceiveBeginPlay`
  (`KismetSystemLibrary.K2_SetTimer` null "TrySpawnNextInbound" 0.2 true))

(event `self.InboundTrigger.OnComponentBeginOverlap`
  (params (OverlappedComponent :type "PrimitiveComponent Object Reference") (OtherActor :type "Actor Object Reference") (OtherComp :type "PrimitiveComponent Object Reference") (OtherBodyIndex :type Integer) (bFromSweep :type Boolean) (SweepResult :type "HitResult Structure (by ref)"))
  (cast `/Game/Warehouse/BP_Pallet` OtherActor)
  (`KismetSystemLibrary.Delay` 1.0)
  (set `self.InboundSlotUsed` false)
  (if (`|EnumEquality` (`/Game/Warehouse/BP_StackerCrane_02.InboundMoveType` (`self.Crane`)) "NewEnumerator4")
    (`/Game/Warehouse/BP_StackerCrane_02.InboundProcess` (`self.Crane`))))

(fn `RequestInbound`
  (bind _crane (`self.Crane`))
  (if (`|EnumEquality` (`/Game/Warehouse/BP_StackerCrane_02.Jobtype` (`self.Crane`)) "NewEnumerator0")
    (set `/Game/Warehouse/BP_StackerCrane_02.Jobtype` "NewEnumerator1" _crane)
    (set `/Game/Warehouse/BP_StackerCrane_02.OutboundMoveType` "NewEnumerator0" _crane)
    (else
      (set `self.PendingInboundCount` (+ (`self.PendingInboundCount`) 1)))))

(fn `TrySpawnNextInbound`
  (if (> (`self.PendingInboundCount`) 0)
    (if (`self.InboundSlotUsed`)
      _
      (elif (`|EnumEquality` (`/Game/Warehouse/BP_StackerCrane_02.InboundMoveType` (`self.Crane`)) "NewEnumerator4")
        (set `self.PendingInboundCount` (- (`self.PendingInboundCount`) 1))
        (set `self.InboundSlotUsed` true)
        (bind _returnvalue (`|SpawnActorFromClass` "/Game/Warehouse/BP_Pallet.BP_Pallet_C" (`KismetMathLibrary.MakeTransform` (`SceneComponent.K2_GetComponentLocation` (`self.SpawnPoint`))) "Undefined" "MultiplyWithRoot" null null))
        (`/Game/Warehouse/BP_Pallet.MoveToInbound` _returnvalue (`SceneComponent.K2_GetComponentLocation` (`self.InboundPoint`)))))))

(fn `UserConstructionScript`)